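; Custom PCG Blueprint element that picks a random subset of points from each spatial input, capped at NumberOfPoints.
; Each input converts to point data, and a shuffled index array chooses points, whose density is set to 10.
; The selection replaces that data's points and is output with original tags and pin.
; The shuffle is unseeded, and the index and selection arrays are never cleared between inputs.
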(fn ExecutewithContext
  (params (InContext :type PCG%20Context%20Structure%20%28by%20ref%29) (Input :type PCG%20Data%20Collection%20Structure%20%28by%20ref%29))
  (bind _indexmap (Variables|Default|GetIndexMap))
  (bind _returnvalue (Class|PCGDataFunctionLibrary|GetInputs Input))
  (for _array_element _returnvalue
    (Variables|Default|SetPin (.Pin (Utilities|Struct|BreakPCGTaggedData _array_element)))
    (Variables|Default|SetTags (.Tags (Utilities|Struct|BreakPCGTaggedData _array_element)))
    (bind _aspcgspatial_data (Utilities|Casting|CastToPCGSpatialData (.Data (Utilities|Struct|BreakPCGTaggedData _array_element))))
    (bind _output_get (Variables|Default|SetPCGPointData (SpatialData|ToPointDatawithContext _aspcgspatial_data InContext)))
    (bind _output_get_2 (Variables|Default|SetPCGPoints (SpatialData|GetPoints _output_get)))
    (bind _output_get_3 (Variables|Default|SetPointCount (Utilities|Array|Length _output_get_2)))
    (if (<= _output_get_3 (Variables|Default|GetNumberOfPoints))
      (Variables|Default|SetSelectQuantity (Variables|Default|GetPointCount))
      (else
        (Variables|Default|SetSelectQuantity (Variables|Default|GetNumberOfPoints))))
    (Variables|Default|SetSelectQuantity (- (Variables|Default|GetSelectQuantity) 1))
    (for _index (range 0 (- (Variables|Default|GetPointCount) 1))
      (Utilities|Array|Add _indexmap _index))
    (Utilities|Array|Shuffle _indexmap)
    (for _index_2 (range 0 (Variables|Default|GetSelectQuantity))
      (bind _structout (Utilities|Struct|SetmembersinPCGPoint (Utilities|Array|Get(acopy) (Variables|Default|GetPCGPoints) (Utilities|Array|Get(acopy) (Variables|Default|GetIndexMap) _index_2)) 1e+01))
      (Utilities|Array|Add (Variables|Default|GetSelectedPoints) _structout))
    (SpatialData|SetPoints (Variables|Default|GetPCGPointData) (Variables|Default|GetSelectedPoints))
    (Utilities|Array|Add (Variables|Default|GetOutTaggedData) (Utilities|Struct|MakePCGTaggedData (Variables|Default|GetPCGPointData) (Variables|Default|GetTags) (Variables|Default|GetPin))))
  (return (Utilities|Struct|MakePCGDataCollection (Variables|Default|GetOutTaggedData))))